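; Automatic rifle that fires paintballs while the trigger is held.
; PullTrigger fires at once through a DoOnce gate, then starts a looping timer on Fire at the RoundsPerSecond rate.
; Each shot spawns a BP_PaintBall at ProjectileSpawnPoint and plays the rifle sound at the actor's location.
; ReleaseTrigger clears the timer and resets the gate, so re-pulling fires immediately without waiting out the interval.
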(event Custom|PullTrigger
  ;[1 1 1] Fire
  (Utilities|FlowControl|DoOnce false
    (:Completed
      (CallFunction|Fire)
      (Utilities|Time|SetTimerbyFunctionName 0 "Fire" (/ 1.0 (Variables|Default|GetRoundsPerSecond)) true))))

(event Custom|ReleaseTrigger
  ;[1 1 1] Fire
  (Utilities|Time|ClearTimerbyFunctionName 0 "Fire")
  (Utilities|FlowControl|DoOnce false) ; enters at Reset
)

(event Custom|Fire
  ;[1 1 1] Fire
  (Game|SpawnActorfromClass "/Game/Splat/Weapons/PaintBall/BP_PaintBall.BP_PaintBall_C" (Transformation|GetWorldTransform (Variables|Default|GetProjectileSpawnPoint)) "Undefined" 0 0)
  (Audio|PlaySoundatLocation "/Game/Splat/Weapons/Rifle/Audio/RifleFire.RifleFire" (Transformation|GetActorLocation) "0, 0, 0" 1.0 1.0 0.0 0 0 0))

(fn ConstructionScript)