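; BP_Rifle is an automatic paintball rifle weapon that fires while the trigger is held.
; PullTrigger fires once, then loops Fire on a timer set by RoundsPerSecond, with a DoOnce that ReleaseTrigger resets as it clears the timer.
; Each shot checks ammo on the first controller's BP_GamePlay_PS, spawns a BP_PaintBall at the spawn point, plays a sound and reduces ammo, or prints an out-of-ammo message.
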(event Custom|PullTrigger
  ;[1 1 1] Fire
  (bind _asbp_base_player (Utilities|Casting|CastToBP_BasePlayer (Game|GetPlayerCharacter 0)))
  (Variables|Default|SetPlayer _asbp_base_player)
  (if true
    (Utilities|FlowControl|DoOnce false
      (:Completed
        (CallFunction|Fire)
        (Utilities|Time|SetTimerbyFunctionName 0 "Fire" (/ 1.0 (Variables|Default|GetRoundsPerSecond)) true)))))

(event Custom|ReleaseTrigger
  ;[1 1 1] Fire
  (Utilities|Time|ClearTimerbyFunctionName 0 "Fire")
  (Utilities|FlowControl|DoOnce false) ; enters at Reset
)

(event Custom|Fire
  ;[1 1 1] Fire
  (bind _asbp_game_play_ps (Utilities|Casting|CastToBP_GamePlay_PS (Variables|/Script/Engine.Controller|GetPlayerState (Game|GetPlayerController 0)))
    (:then
      (if (> (Variables|/Game/Whoopensocker/Core/GamePlay/BP_GamePlay_PS.BP_GamePlay_PS_C|GetCurrentAmmo _asbp_game_play_ps) 0)
        (Game|SpawnActorfromClass "/Game/Whoopensocker/Weapons/PaintBall/BP_PaintBall.BP_PaintBall_C" (Transformation|GetWorldTransform (Variables|Default|GetProjectileSpawnPoint)) "Undefined" 0 0)
        (Audio|PlaySoundatLocation "/Game/Whoopensocker/Weapons/Rifle/Audio/RifleFire.RifleFire" (Transformation|GetActorLocation) "0, 0, 0" 1.0 1.0 0.0 0 0 0)
        (Default|ReduceAmmo _asbp_game_play_ps)
        (else
          (Development|PrintString "Out of Ammo"))))
    (:CastFailed
      (Development|PrintString "FAILED: Cast to BP_GamePlay_PS" true true "(R=1.000000,G=0.000000,B=0.000000,A=1.000000)" 1e+01))))

(fn ConstructionScript)