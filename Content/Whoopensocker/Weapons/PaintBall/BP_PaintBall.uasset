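; BP_PaintBall is a paintball projectile that bursts into colored paint where it hits.
; On hit it destroys itself and spawns a paint explosion particle at the impact point, tinted with player 0's PaintColor from BP_BasePlayer.
; It then attaches a splatter decal to the struck component and bone, using a dynamic material in the same color, aligned to the impact normal with random roll for variety.
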(event Collision|EventHit
  (params (MyComp :type Primitive%20Component%20Object%20Reference) (Other :type Actor%20Object%20Reference) (OtherComp :type Primitive%20Component%20Object%20Reference) (bSelfMoved :type Boolean) (HitLocation :type Vector :default "0, 0, 0") (HitNormal :type Vector :default "0, 0, 0") (NormalImpulse :type Vector :default "0, 0, 0") (Hit :type Hit%20Result%20Structure%20%28by%20ref%29))
  (bind (_bblockinghit _binitialoverlap _time _distance _location _impactpoint _normal _impactnormal _physmat _hitactor _hitcomponent _hitbonename) (Collision|BreakHitResult Hit))
  (bind _returnvalue (Math|Conversions|RotationFromXVector _impactnormal))
  (bind (_roll _pitch _yaw) (Math|Rotator|BreakRotator _returnvalue))
  ;[1 1 1] PaintBall Hit
  (Variables|Default|SetHitComponent OtherComp)
  (Actor|DestroyActor (Components|GetOwner MyComp))
  (bind _returnvalue_2 (Effects|SpawnEmitteratLocation "/Game/Whoopensocker/Effects/Particles/PS_PaintExplosion.PS_PaintExplosion" _impactpoint))
  (bind _asbp_base_player (Utilities|Casting|CastToBP_BasePlayer (Game|GetPlayerCharacter 0)))
  (Effects|Components|ParticleSystem|SetColorParameter _returnvalue_2 "InstanceColorScaleOverLife" (Math|Conversions|ToLinearColor(Color) (Variables|/Game/Whoopensocker/Characters/Player/BP_BasePlayer.BP_BasePlayer_C|GetPaintColor _asbp_base_player)))
  (bind _returnvalue_3 (Rendering|Material|CreateDynamicMaterialInstance "/Game/Whoopensocker/Core/Materials/M_PaintSplatter.M_PaintSplatter" "None" :!class /Script/Engine.KismetMaterialLibrary))
  (Rendering|Material|SetVectorParameterValue _returnvalue_3 "PaintColor" (Math|Conversions|ToLinearColor(Color) (Variables|/Game/Whoopensocker/Characters/Player/BP_BasePlayer.BP_BasePlayer_C|GetPaintColor _asbp_base_player)) :!class /Script/Engine.MaterialInstanceDynamic)
  (Class|GameplayStatics|SpawnDecalAttached _returnvalue_3 "15.000000,15.000000,15.000000" _hitcomponent _hitbonename _impactpoint (Math|Rotator|MakeRotator (Math|Random|RandomFloatinRange 0.0 3.6e+02) _pitch _yaw) "KeepWorldPosition" 0.0))

(fn ConstructionScript)