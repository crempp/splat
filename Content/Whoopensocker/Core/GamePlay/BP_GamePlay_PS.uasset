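; BP_GamePlay_PS is the gameplay Player State, holding a player's paint cover, ammo and weapon name.
; On BeginPlay the authority sets the starting values, while a remote instance casts the first Player Controller to BP_GamePlay_PC and tells it to set up the HUD.
; A ReduceAmmo event subtracts the given amount from current ammo, treating zero as a decrement of one.
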(event Custom|ReduceAmmo
  (params (Amount :type Integer))
  ;[1 1 1] Reduce Player Ammo
  (if (== Amount 0)
    (Math|Integer|DecrementInt (Variables|Default|GetCurrentAmmo))
    (else
      (Variables|Default|SetCurrentAmmo (- (Variables|Default|GetCurrentAmmo) Amount)))))

(event EventBeginPlay
  ;[1 1 1] Player State Setup
  (Networking|SwitchHasAuthority
    (:Authority
      ;;[1 1 1] Set initial values
      (Variables|Default|SetPaintCover 0.0)
      (Variables|Default|SetMaxPaintCover 1e+02)
      (Variables|Default|SetCurrentAmmo 90)
      (Variables|Default|SetMaxAmmo 90)
      (Variables|Default|SetWeaponName "A31 Rapid Fire Rifle"))
    (:Remote
      ;;[1 1 1] Tell the Player Controller to setup the HUD
      (bind _asbp_game_play_pc (Utilities|Casting|CastToBP_GamePlay_PC (Game|GetPlayerController 0)))
      (Default|SetupHUD _asbp_game_play_pc))))

(fn ConstructionScript)