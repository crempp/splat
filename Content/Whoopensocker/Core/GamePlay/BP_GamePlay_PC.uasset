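; BP_GamePlay_PC is the gameplay player controller, handling player spawn setup and multiplayer text chat.
; On BeginPlay the local controller loads saved player settings and passes them to the server, which has BP_GamePlay_GM spawn the chosen character, then calls chat widget setup.
; Chat messages are relayed through the game mode's controller list, updating each player's chat window with sender name and text.
; The T key toggles the mouse cursor for chatting.
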(event Custom|PassCharacterInfoToServer
  (params (PlayerSettingsInfo :type S%20Player%20Info%20Structure))
  ;[0.2865 0.2608 0.04097] Setup
  ;;[1 1 1] Pass Character Info, Respawn, Setup Chat Window
  (Variables|Default|SetPlayer%20Settings PlayerSettingsInfo)
  (bind _asbp_game_play_gm (Utilities|Casting|CastToBP_GamePlay_GM (Game|GetGameMode)))
  (Default|InitialPlayerSpawn _asbp_game_play_gm (.myplayercharacter (Variables|Default|GetPlayer%20Settings)) self)
  (CallFunction|SetupChatWindow))

(event Custom|SetupChatWindow
  ;[1 1 1] Creat GamePlay Chat, Add to Viewport
  (bind _returnvalue (UserInterface|CreateWidget "/Game/Whoopensocker/UI/CustomWidgets/WBP_GamePlayChat.WBP_GamePlayChat_C"))
  (bind _output_get (Variables|Default|SetWB_GamePlayChat _returnvalue))
  (UserInterface|Viewport|AddtoViewport _output_get 0))

(event Custom|GetChatMessage
  (params (TextToSend :type Text))
  ;[0.2083 0.9901 1] Chat
  ;;[1 1 1] Process Incoming Chats on Server and Send to Clients
  (Variables|Default|SetSenderText TextToSend)
  (Variables|Default|SetSenderName (.myplayername (Variables|Default|GetPlayer%20Settings)))
  (bind _asbp_game_play_gm (Utilities|Casting|CastToBP_GamePlay_GM (Game|GetGameMode)))
  (for _array_element (Variables|/Game/Whoopensocker/Core/GamePlay/BP_GamePlay_GM.BP_GamePlay_GM_C|GetAllPlayerControllers _asbp_game_play_gm)
    (bind _asbp_game_play_pc (Utilities|Casting|CastToBP_GamePlay_PC _array_element))
    (CallFunction|UpdateChat _asbp_game_play_pc (Variables|Default|GetSenderName) (Variables|Default|GetSenderText))))

(event Custom|UpdateChat
  (params (SenderName :type Text) (SenderText :type Text))
  ;[0.2083 0.9901 1] Chat
  ;;[1 1 1] Update Chat on Client
  (Default|UpdateChatWindow (Variables|/Game/Whoopensocker/UI/CustomWidgets/WBP_GamePlayChat.WBP_GamePlayChat_C|GetGamePlayChat (Variables|Default|GetWB_GamePlayChat)) SenderName SenderText))

(event EventBeginPlay
  ;[0.2865 0.2608 0.04097] Setup
  ;;[1 1 1] Load Player Info and Pass to Server
  (if (Pawn|IsLocalController)
    (Viewport|RemoveAllWidgets)
    (CallFunction|LoadGame)
    (CallFunction|PassCharacterInfotoServer (Variables|Default|GetPlayer%20Settings))))

(event Input|KeyboardEvents|T
  (params (Key :type Key%20Structure))
  ;[1 1 1] T to Type Chat
  (:Pressed
    (Utilities|FlowControl|FlipFlop
      (:A
        (Variables|Default|SetbShowMouseCursor true))
      (:B
        (Variables|Default|SetbShowMouseCursor false)))))

(fn ConstructionScript)

(fn LoadGame
  (bind _returnvalue (SaveGame|LoadGamefromSlot (Variables|Default|GetPlayerSettingsSave)))
  (bind _asbp_player_save_game (Utilities|Casting|CastToBP_PlayerSaveGame _returnvalue))
  (Variables|Default|SetPlayer%20Settings (Variables|/Game/Whoopensocker/Core/BP_PlayerSaveGame.BP_PlayerSaveGame_C|GetSPlayerInfo _asbp_player_save_game)))